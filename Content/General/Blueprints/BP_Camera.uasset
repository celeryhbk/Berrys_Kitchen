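; Camera Blueprint that also holds the item inventory and handles touch input for dialogue.
; A touch press advances the DialoguePlayer to its next row, AddItem appends to the Inventory array, and a debug F key prints its contents.
; TryCraftFromInventory is an empty stub: its unconnected draft looks up fixed potion and poison row names in DT_CraftingRecipes without comparing ingredients, and most AddItem calls lack an item.
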(event Collision|EventActorBeginOverlap
  (params (OtherActor :type Actor%20Object%20Reference)))

(event EventTick
  (params (DeltaSeconds :type Float%20%28single-precision%29)))

(event EventAddItem
  (params (Item :type Texture%202D%20Object%20Reference))
  (Utilities|Array|Add (Variables|Default|GetInventory) Item))

(event Input|KeyboardEvents|DebugKeyF
  (params (Key :type Key%20Structure :default "None") (ActionValue :type Input%20Action%20Value%20Structure))
  (:Pressed
    (for _array_element (Variables|Default|GetInventory)
      (Development|PrintString (Utilities|GetDisplayName _array_element)))))

(event Input|TouchEvents|Touch1
  (params (Key :type Key%20Structure :default "None"))
  (bind _dialogue_player (Variables|Default|GetDialogue_Player))
  (:Pressed
    (Utilities|IsValid _dialogue_player
      (:Is%20Valid
        (Default|NextRowViaPlayer _dialogue_player)))))

(fn ConstructionScript)

(fn TryCraftfromInventory)