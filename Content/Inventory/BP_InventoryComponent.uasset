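; Inventory component that holds items in a fixed-size array of slot structs with stack counts.
; BeginPlay builds InventorySize slots.
; AddItem raises a matching stack below the item's max size, though that write sets HasItem false, or otherwise writes a new stack upon finding an empty slot.
; RemoveItem decrements or clears the found slot, and AddIngredient adds a preset ingredient through AddItem.
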(event `self.ReceiveBeginPlay`
  (`self.InventoryConstructor`))

(fn `AddIngredient`
  (`self.AddItem` "/Game/Inventory/Item_Ingredient1.Item_Ingredient1"))

(fn `AddItem`
  (params (ItemToAdd :type "/Game/Inventory/BP_Item Object Reference"))
  (returns (HasFoundSlot1 :type Boolean))
  (locals (HasFoundSlot :type Boolean))
  (bind _hasfoundslot (`local.HasFoundSlot`))
  (for (_array_element _array_index) (`self.Inventory`)
    (bind (_hasitem _stacksize _itemassets) (break `/Game/Inventory/STR_InventorySlot` _array_element))
    (if _hasitem
      (if (== ItemToAdd _itemassets)
        (if (< _stacksize (`/Game/Inventory/BP_Item.MaxStackSize` ItemToAdd))
          (`KismetArrayLibrary.Array_Set` (`self.Inventory`) _array_index (make `/Game/Inventory/STR_InventorySlot` false (+ _stacksize 1) ItemToAdd))
          (set `local.HasFoundSlot` true)
          (break)))))
  (if _hasfoundslot
    (return _hasfoundslot)
    (else
      (for _array_element_2 (`self.Inventory`)
        (if (not (`.HasItem_1_FE991463410FE08A73956F802CDE2427` (break `/Game/Inventory/STR_InventorySlot` _array_element_2)))
          (`KismetArrayLibrary.Array_Set` (`self.Inventory`) 0 (make `/Game/Inventory/STR_InventorySlot` true 1 ItemToAdd))
          (set `local.HasFoundSlot` true)
          (break)))
      (return (`local.HasFoundSlot`)))))

(fn `InventoryConstructor`
  (bind _inventory (`self.Inventory`))
  (`KismetArrayLibrary.Array_Clear` _inventory)
  (for _ (range (`self.Inventory Size`))
    (`KismetArrayLibrary.Array_Add` _inventory)))

(fn `RemoveItem`
  (params (ItemToFind :type "/Game/Inventory/STR_InventorySlot Structure (by ref)"))
  (bind _inventory (`self.Inventory`))
  (bind _output (`|GetArrayItem` _inventory (`KismetArrayLibrary.Array_Find` _inventory ItemToFind)))
  (bind (_hasitem _stacksize _itemassets) (break `/Game/Inventory/STR_InventorySlot` _output))
  (if (> _stacksize 1)
    (bind _result (`/Engine/EditorBlueprintResources/StandardMacros.DecrementInt` _stacksize)
      (:`  `
        (`|VariableSetRef` _output (make `/Game/Inventory/STR_InventorySlot` true _result _itemassets))))
    (else
      (`|VariableSetRef` _output (make `/Game/Inventory/STR_InventorySlot` false))))
  (return))