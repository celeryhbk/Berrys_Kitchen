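; BP_Contractor is a customer actor for the counter scene that animates into frame when play begins and animates away when despawned.
; A timeline curve drives the root component's X location on entry, while both animations hold the scale at half size.
; DespawnActor plays a second timeline for the exit, whose update also starts a three-second delay before the actor destroys itself.
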(event `self.ReceiveBeginPlay`
  ;[1 1 1] Customer moves into Frame
  (bind (_direction _customanim) (`Timeline|Timeline`)
    (:`Update`
      (`|ExecutionSequence`
        (:`then_0`
          (`SceneComponent.K2_SetRelativeLocation` (`self.DefaultSceneRoot`) (`KismetMathLibrary.MakeVector` _customanim) false false)
          (`SceneComponent.SetRelativeScale3D` (`self.DefaultSceneRoot`) (`KismetMathLibrary.Conv_DoubleToVector` 0.5)))))))

(event `DespawnActor`
  (bind (_direction _customanim _customanimscale _location_y _animdespawn) (`Timeline|Timeline_0`)
    (:`Update`
      (`SceneComponent.K2_SetRelativeLocation` (`self.DefaultSceneRoot`) (`KismetMathLibrary.MakeVector` _animdespawn) false false)
      (`SceneComponent.SetRelativeScale3D` (`self.DefaultSceneRoot`) (`KismetMathLibrary.Conv_DoubleToVector` 0.5))
      (`KismetSystemLibrary.Delay` 3.0)
      (`self.K2_DestroyActor`))))

(fn `UserConstructionScript`)