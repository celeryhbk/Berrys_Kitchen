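; First customer actor at the counter, holding a repeatable dialogue shown in a UMG widget.
; Each DialogueEvent call, meant for Space presses, advances TalkIndex through the Dialogue array and writes that line to WP_FirstCustomer_Dialogue.
; Once the index exceeds the array length, it removes the widget and resets for replay.
; A move-into-frame timeline driving location and scale exists but is never triggered.
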(event `self.ReceiveBeginPlay`)

(event `/Game/Counter/Blueprints/BPI_Berrys.Dialogue_Event`
  (`/Engine/EditorBlueprintResources/StandardMacros.IncrementInt` (`self.TalkIndex`) ; Everytime we press "Space" we're adding\n to the Index to advance in the Array
    (:`  `
      (if (<= (`self.TalkIndex`) (`KismetArrayLibrary.Array_Length` (`self.Dialogue`)))
        ;[1 0.5961 0.2784] Adding the Dialogue Widget to the Viewport (if it hasn't been done before)
        (bind _returnvalue (`|CreateWidget` "/Game/Counter/Blueprints/WIdgets/WP_FirstCustomer_Dialogue.WP_FirstCustomer_Dialogue_C" (`GameplayStatics.GetPlayerController` 0)))
        (`self.UI_Dialogue`
          (:`then`
            _)
          (:`else`
            (bind _output_get (set `self.UI_Dialogue` _returnvalue))
            (`UserWidget.AddToViewport` _output_get 0)))
        ;[1 0.5961 0.2784] setting our Array Text as Dialogue
        (`TextBlock.SetText` (`/Game/Counter/Blueprints/WIdgets/WP_FirstCustomer_Dialogue.First_Customer_Dialogue` (`self.UI_Dialogue`)) (`KismetTextLibrary.Conv_StringToText` (`|GetArrayItem` (`self.Dialogue`) (`self.TalkIndex`))))
        (else
          (`Widget.RemoveFromParent` (`self.UI_Dialogue`)) ; If the Index is bigger, we remove it \nfrom the Viewport to end the conversation
          ;[1 0.5961 0.2784] Making the Dialogue repeatable
          (set `self.TalkIndex` -1)
          (set `self.UI_Dialogue` null))))))

(fn `GetActorTransform`
  (returns (OutActorTransforms :type "Transform Structure"))
  (return))

(fn `UserConstructionScript`)